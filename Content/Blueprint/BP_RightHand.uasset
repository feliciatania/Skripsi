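; Right-hand VR hand Blueprint built on an OculusHand component, extending a parent class that supplies any BeginPlay behavior.
; The construction script attaches Thumb, Index, Middle, Ring and Pinky components to the matching right-hand fingertip bone sockets, keeping relative transforms.
; Nodes that would assign a low-res physics asset and initialize hand physics are present but disconnected, so they never run.
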(event `self.ReceiveBeginPlay`
  (`parent.ReceiveBeginPlay`))

(fn `UserConstructionScript`
  (`parent.UserConstructionScript`)
  (`SceneComponent.K2_AttachToComponent` (`self.Thumb`) (`self.OculusHand`) "b_r_thumb3" "KeepRelative" "KeepRelative" "KeepRelative" true)
  (`SceneComponent.K2_AttachToComponent` (`self.Index`) (`self.OculusHand`) "b_r_index3" "KeepRelative" "KeepRelative" "KeepRelative" true)
  (`SceneComponent.K2_AttachToComponent` (`self.Middle`) (`self.OculusHand`) "b_r_middle3" "KeepRelative" "KeepRelative" "KeepRelative" true)
  (`SceneComponent.K2_AttachToComponent` (`self.Ring`) (`self.OculusHand`) "b_r_ring3" "KeepRelative" "KeepRelative" "KeepRelative" true)
  (`SceneComponent.K2_AttachToComponent` (`self.Pinky`) (`self.OculusHand`) "b_r_pinky3" "KeepRelative" "KeepRelative" "KeepRelative" true))