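; Collision-box actor that tallies and removes gem pickups (permata) inside its capsule, apparently for exchanging them for point cards (kartu point).
; CheckPermata counts overlapping BP_PickupCube actors by tag into an SPermata struct, though only sapphire is tested on each cube; emerald and ruby are tested on the box itself.
; DestroyPermata destroys the first overlapping cube, then returns.
; The event graph has no logic.
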(event `self.ReceiveBeginPlay`)

(fn `CheckPermata`
  (returns (Permatas :type "/Game/Blueprint/S_Permata Structure"))
  (bind _overlappingactors (`PrimitiveComponent.GetOverlappingActors` (`self.Capsule`) "/Game/Blueprint/BP_PickupCube.BP_PickupCube_C"))
  (set `self.count` (`KismetArrayLibrary.Array_Length` _overlappingactors))
  (set `self.Sapphire` 0)
  (set `self.Emerald` 0)
  (set `self.Ruby` 0)
  (for _array_element _overlappingactors
    (if (`self.ActorHasTag` _array_element "sapphire")
      (`/Engine/EditorBlueprintResources/StandardMacros.IncrementInt` (`self.Sapphire`))
      (elif (`self.ActorHasTag` "emerald")
        (`/Engine/EditorBlueprintResources/StandardMacros.IncrementInt` (`self.Emerald`))
        (elif (`self.ActorHasTag` "ruby")
          (`/Engine/EditorBlueprintResources/StandardMacros.IncrementInt` (`self.Ruby`))))))
  (bind _output_get (set `self.SPermata` (make `/Game/Blueprint/S_Permata` (`self.Sapphire`) (`self.Emerald`) (`self.Ruby`))))
  (return _output_get))

(fn `DestroyPermata`
  (for _array_element (`PrimitiveComponent.GetOverlappingActors` (`self.Capsule`) "/Game/Blueprint/BP_PickupCube.BP_PickupCube_C")
    (`self.K2_DestroyActor` _array_element)
    (return)))

(fn `UserConstructionScript`)