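; BP_VRHandPawn is a VR pawn for recording named hand gestures from the left and right hands.
; On BeginPlay it sets the tracking origin to floor level.
; The R and L keys call RecordGesture with GestureName on RightHand or LeftHand respectively, then print a confirmation.
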(event `self.ReceiveBeginPlay`
  (`HeadMountedDisplayFunctionLibrary.SetTrackingOrigin` "Floor"))

(event `Key|R`
  (params (Key :type "Key Structure"))
  (:`Pressed`
    (`/Game/Blueprint/BPC_OculusHand.RecordGesture` (`self.RightHand`) (`self.GestureName`))
    (`KismetSystemLibrary.PrintString` "Recorded Right")))

(event `Key|L`
  (params (Key :type "Key Structure"))
  (:`Pressed`
    (`/Game/Blueprint/BPC_OculusHand.RecordGesture` (`self.LeftHand`) (`self.GestureName`))
    (`KismetSystemLibrary.PrintString` "Recorded Left")))

(event `Key|D`
  (params (Key :type "Key Structure")))

(fn `UserConstructionScript`)