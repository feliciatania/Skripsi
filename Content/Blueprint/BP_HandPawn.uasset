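; BP_HandPawn is a VR pawn that provides left and right hands and displays their recognised gestures.
; On BeginPlay it sets a floor tracking origin, then spawns BP_Hand and BP_RightHand and attaches both to itself.
; It binds to each hand's OnGestureRecognised event and caches the WB_CurGesture widget from each side's widget component.
; Per-hand handlers write the gesture name into the matching widget's CurrentGesture.
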(event `self.ReceiveBeginPlay`
  (bind _returnvalue (`KismetMathLibrary.MakeTransform` (0.0 0.0 0.0)))
  (`|ExecutionSequence`
    (:`then_0`
      (`HeadMountedDisplayFunctionLibrary.SetTrackingOrigin` "Floor")
      (`|ExecutionSequence`
        (:`then_0`
          (bind _returnvalue_2 (`|SpawnActorFromClass` "/Game/Blueprint/BP_Hand.BP_Hand_C" _returnvalue "Undefined" "OverrideRootScale" self "Left" null))
          (bind _output_get (set `self.LeftHand` _returnvalue_2))
          (`self.K2_AttachToActor` _output_get self "None" "SnapToTarget" "SnapToTarget" "KeepWorld" false))
        (:`then_1`
          (bind _returnvalue_3 (`|SpawnActorFromClass` "/Game/Blueprint/BP_RightHand.BP_RightHand_C" _returnvalue "Undefined" "OverrideRootScale" self "Right" null))
          (bind _output_get_2 (set `self.RightHand` _returnvalue_3))
          (`self.K2_AttachToActor` _output_get_2 self "None" "SnapToTarget" "SnapToTarget" "KeepWorld" false))))
    (:`then_1`
      (`|ExecutionSequence`
        (:`then_0`
          (add `/Game/Blueprint/BP_Hand.onGestureRecognised` (`self.LeftHand`) (`|CreateDelegate` :!event `GestureRecognisedLeft`))
          (add `/Game/Blueprint/BP_Hand.onGestureRecognised` (`self.RightHand`) (`|CreateDelegate` :!event `GestureRecognisedRight`)))
        (:`then_1`
          (bind _aswb_cur_gesture (cast `/Game/Blueprint/WB_CurGesture` (`WidgetComponent.GetUserWidgetObject` (`self.Widget Left`))))
          (set `self.As WB Cur Gesture Left` _aswb_cur_gesture)
          (bind _aswb_cur_gesture_2 (cast `/Game/Blueprint/WB_CurGesture` (`WidgetComponent.GetUserWidgetObject` (`self.Widget Right`))))
          (set `self.As WB Cur Gesture Right` _aswb_cur_gesture_2))))))

(event `GestureRecognisedLeft`
  (params (GestureName :type String))
  (set `/Game/Blueprint/WB_CurGesture.CurrentGesture` GestureName (`self.As WB Cur Gesture Left`)))

(event `GestureRecognisedRight`
  (params (GestureName :type String))
  (set `/Game/Blueprint/WB_CurGesture.CurrentGesture` GestureName (`self.As WB Cur Gesture Right`)))

(fn `UserConstructionScript`)