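; BP_CollisonBoxKartu is a card slot trigger that requests a replacement card when its box is empty.
; A looping one-second timer started on BeginPlay drives the check, with CheckCollision acting only on the server.
; IsPointCard selects whether it looks for overlapping BP_KartuPoin or BP_KartuPedagang (merchant) actors.
; With none found, it calls the matching spawn function on BP_GameStateBase, passing its slot Id.
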(event `self.ReceiveBeginPlay`
  (`KismetSystemLibrary.K2_SetTimerDelegate` (`|CreateDelegate` :!event `CheckCollision`) 1.0 true))

(event `CheckCollision`
  (`/Engine/EditorBlueprintResources/ActorMacros.Switch Has Authority`
    (:`Authority`
      (if (`self.isPointCard`)
        (if (== (`KismetArrayLibrary.Array_Length` (`PrimitiveComponent.GetOverlappingActors` (`self.Box`) "/Game/Blueprint/Game/BP_KartuPoin.BP_KartuPoin_C")) 0)
          (bind _asbp_game_state_base (cast `/Game/Blueprint/BP_GameStateBase` (`GameplayStatics.GetGameState`)))
          (`/Game/Blueprint/BP_GameStateBase.SpawnKartuPoin` _asbp_game_state_base (`self.id`)))
        (elif (== (`KismetArrayLibrary.Array_Length` (`PrimitiveComponent.GetOverlappingActors` (`self.Box`) "/Game/Blueprint/Game/BP_KartuPedagang.BP_KartuPedagang_C")) 0)
          (bind _asbp_game_state_base_2 (cast `/Game/Blueprint/BP_GameStateBase` (`GameplayStatics.GetGameState`)))
          (`/Game/Blueprint/BP_GameStateBase.SpawnKartuPedagang` _asbp_game_state_base_2 (`self.id`)))))))

(fn `UserConstructionScript`)