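; Right-hand VR hand Blueprint, a child class that supplies right-side bone names and attachments for an Oculus hand.
; The construction script attaches five finger components to the third bone of each finger and moves the arc direction and spline to the Teleport socket.
; It also fills the finger bone and fingertip marker name arrays.
; BeginPlay only calls the parent; the hand physics setup nodes are unconnected and never run.
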(event `self.ReceiveBeginPlay`
  (`parent.ReceiveBeginPlay`))

(fn `UserConstructionScript`
  (`parent.UserConstructionScript`)
  (`SceneComponent.K2_AttachToComponent` (`self.Thumb`) (`self.OculusHand`) "b_r_thumb3" "KeepRelative" "KeepRelative" "KeepRelative" true)
  (`SceneComponent.K2_AttachToComponent` (`self.Index`) (`self.OculusHand`) "b_r_index3" "KeepRelative" "KeepRelative" "KeepRelative" true)
  (`SceneComponent.K2_AttachToComponent` (`self.Middle`) (`self.OculusHand`) "b_r_middle3" "KeepRelative" "KeepRelative" "KeepRelative" true)
  (`SceneComponent.K2_AttachToComponent` (`self.Ring`) (`self.OculusHand`) "b_r_ring3" "KeepRelative" "KeepRelative" "KeepRelative" true)
  (`SceneComponent.K2_AttachToComponent` (`self.Pinky`) (`self.OculusHand`) "b_r_pinky3" "KeepRelative" "KeepRelative" "KeepRelative" true)
  (`SceneComponent.K2_SetWorldLocation` (`self.ArcDirection`) (`SceneComponent.GetSocketLocation` (`self.OculusHand`) "Teleport") false false)
  (`SceneComponent.K2_SetWorldLocation` (`self.ArcSpline`) (`SceneComponent.GetSocketLocation` (`self.OculusHand`) "Teleport") false false)
  (set `self.HandFingers1` (`|MakeArray` "b_r_thumb1" "b_r_middle1" "b_r_ring1" "b_r_pinky1" "b_r_index1" :!type "Name"))
  (set `self.HandFingers2` (`|MakeArray` "b_r_thumb2" "b_r_middle2" "b_r_ring2" "b_r_pinky2" "b_r_index2" :!type "Name"))
  (set `self.HandFingers3` (`|MakeArray` "b_r_thumb3" "b_r_middle3" "b_r_ring3" "b_r_pinky3" "b_r_index3" :!type "Name"))
  (set `self.FingerTips` (`|MakeArray` "r_thumb_finger_tip_marker" "r_index_finger_tip_marker" "r_middle_finger_tip_marker" "r_ring_finger_tip_marker" "r_pinky_finger_tip_marker" :!type "Name")))