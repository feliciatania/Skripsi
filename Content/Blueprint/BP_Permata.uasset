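; BP_Permata is a grabbable physics actor that BP_MotionController picks up and drops.
; Pickup turns off mesh physics and attaches the root to the given component, optionally snapping to a socket, while Drop detaches it and restores physics.
; Both pass through server-to-clients event chains, named like RPCs, to mirror the physics toggle.
; SetOwnerToNull looks unfinished: it assigns a BP_Permata reference to OwnerPawn and prints a debug string.
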(event `self.ReceiveBeginPlay`)

(event `/Game/Blueprint/PickupActorInterface.Pickup`
  (params (AttachTo :type "SceneComponent Object Reference"))
  (bind _returnvalue (select `bool` (`self.bSnapToSocket?`) :`false` "KeepWorld" :`true` "SnapToTarget" :!type "EAttachmentRule Enum"))
  (if (not (`self.bGrabbed?`))
    (`PrimitiveComponent.SetSimulatePhysics` (`self.StaticMeshComponent`) false)
    (`SceneComponent.K2_AttachToComponent` (`self.RootComponent`) AttachTo (select `bool` (`self.bSnapToSocket?`) :`true` (`self.SnapSocket`)) _returnvalue _returnvalue "KeepRelative" false)
    (set `self.bGrabbed?` true)
    (`self.onGrabServer`)))

(event `/Game/Blueprint/PickupActorInterface.Drop`
  (`PrimitiveComponent.SetSimulatePhysics` (`self.StaticMeshComponent`) true)
  (`self.K2_DetachFromActor` "KeepWorld" "KeepWorld" "KeepWorld")
  (set `self.bGrabbed?` false)
  (`self.onReleaseServer`))

(event `onReleaseServer`
  (`self.onReleaseClients`))

(event `onReleaseClients`
  (`PrimitiveComponent.SetSimulatePhysics` (`self.StaticMeshComponent`) true))

(event `onGrabServer`
  (`self.onGrabClients`))

(event `onGrabClients`
  (`PrimitiveComponent.SetSimulatePhysics` (`self.StaticMeshComponent`) false))

(event `EnablePhysic`
  (params (simulate :type Boolean))
  (`PrimitiveComponent.SetSimulatePhysics` (`self.StaticMeshComponent`) simulate))

(event `SetOwnerToNull`
  (set `self.ownerPawn` "BP_Permata")
  (`KismetSystemLibrary.PrintString` "Hello"))

(fn `GetPickupComponent`
  (returns (PickupComponent :type "/Game/Blueprint/BPC_PickupObject Object Reference"))
  (return (`self.PickupObject`)))

(fn `UserConstructionScript`)