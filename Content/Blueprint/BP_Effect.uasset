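; BP_Effect is an effect Blueprint that spawns short-lived fire, water or magic particle emitters at its own location and rotation.
; Three custom events, SpawnFire, SpawnWater and SpawnMagic, each spawn an emitter, wait two seconds, then destroy the component.
; A separate DoOnce gates each event and resets after cleanup, so repeat calls to the same effect are ignored while it plays.
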(event `SpawnFire`
  (`/Engine/EditorBlueprintResources/StandardMacros.DoOnce` false :!label _label
    (:`Completed`
      (bind _returnvalue (`GameplayStatics.SpawnEmitterAtLocation` null (`self.K2_GetActorLocation`) (`self.K2_GetActorRotation`)))
      (`KismetSystemLibrary.Delay` 2.0)
      (`ActorComponent.K2_DestroyComponent` _returnvalue)
      (goto _label :!via `Reset`))))

(event `SpawnWater`
  (`/Engine/EditorBlueprintResources/StandardMacros.DoOnce` false :!label _label_2
    (:`Completed`
      (bind _returnvalue (`GameplayStatics.SpawnEmitterAtLocation` null (`self.K2_GetActorLocation`) (`self.K2_GetActorRotation`)))
      (`KismetSystemLibrary.Delay` 2.0)
      (`ActorComponent.K2_DestroyComponent` _returnvalue)
      (goto _label_2 :!via `Reset`))))

(event `SpawnMagic`
  (`/Engine/EditorBlueprintResources/StandardMacros.DoOnce` false :!label _label_3
    (:`Completed`
      (bind _returnvalue (`GameplayStatics.SpawnEmitterAtLocation` null (`self.K2_GetActorLocation`) (`self.K2_GetActorRotation`)))
      (`KismetSystemLibrary.Delay` 2.0)
      (`ActorComponent.K2_DestroyComponent` _returnvalue)
      (goto _label_3 :!via `Reset`))))

(fn `UserConstructionScript`)