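; BP_CollisonBox is a card slot trigger that requests a new point card (KartuPoin) or merchant card (KartuPedagang) once the slot is empty.
; When BP_HandPawn ends overlap with the Box, IsPointCard selects the card type.
; A Delay loop polls until no card of that type overlaps the Box.
; It then calls the matching spawn function on BP_GameStateBase with the slot's Id.
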(event `self.Box.OnComponentEndOverlap`
  (params (OverlappedComponent :type "PrimitiveComponent Object Reference") (OtherActor :type "Actor Object Reference") (OtherComp :type "PrimitiveComponent Object Reference") (OtherBodyIndex :type Integer))
  (if (== OtherActor "/Game/Blueprint/BP_HandPawn.BP_HandPawn")
    (if (`self.isPointCard`)
      (while (> (`KismetArrayLibrary.Array_Length` (`PrimitiveComponent.GetOverlappingActors` (`self.Box`) "/Game/Blueprint/Game/BP_KartuPoin.BP_KartuPoin_C")) 0)
        (`KismetSystemLibrary.Delay` 0.5))
      (bind _asbp_game_state_base (cast `/Game/Blueprint/BP_GameStateBase` (`GameplayStatics.GetGameState`)))
      (`/Game/Blueprint/BP_GameStateBase.SpawnKartuPoin` _asbp_game_state_base (`self.id`))
      (else
        (while (> (`KismetArrayLibrary.Array_Length` (`PrimitiveComponent.GetOverlappingActors` (`self.Box`) "/Game/Blueprint/Game/BP_KartuPedagang.BP_KartuPedagang_C")) 0)
          (`KismetSystemLibrary.Delay` 0.5))
        (bind _asbp_game_state_base_2 (cast `/Game/Blueprint/BP_GameStateBase` (`GameplayStatics.GetGameState`)))
        (`/Game/Blueprint/BP_GameStateBase.SpawnKartuPedagang` _asbp_game_state_base_2 (`self.id`))))))

(fn `UserConstructionScript`)