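; Player state for a turn-based card and gem game, broadcasting which merchant cards (Kartu Pedagang) and gems (Permata) are enabled.
; After short delays, BeginPlay binds to the game state's turn-start and hand pawn's move dispatchers.
; Turn handling disables gems and enables merchant cards by deck fullness; gem events set sapphire, emerald and ruby flags, optionally by count.
; Only the merchant-card purchase move has an effect; other move branches are empty.
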(event `self.ReceiveBeginPlay`
  (`KismetSystemLibrary.Delay` 0.1)
  (bind _asbp_game_state_base (cast `/Game/Blueprint/BP_GameStateBase` (`GameplayStatics.GetGameState`)))
  (add `/Game/Blueprint/BP_GameStateBase.onPlayerTurnStart` _asbp_game_state_base (`|CreateDelegate` :!event `PlayersTurn`))
  (`KismetSystemLibrary.Delay` 0.1)
  (bind _asbp_hand_pawn (cast `/Game/Blueprint/BP_HandPawn` (`GameplayStatics.GetPlayerCharacter` 0)))
  (add `/Game/Blueprint/BP_HandPawn.onPlayerMoves` _asbp_hand_pawn (`|CreateDelegate` :!event `OnPlayerMoves`)))

(event `self.ReceiveTick`
  (params (DeltaSeconds :type "Float (single-precision)")))

(event `PlayersTurn`
  (params (Player :type "/Game/Blueprint/E_Turn Enum" :default "NewEnumerator0"))
  (`self.EnablePermataSapphire` false)
  (`self.EnablePermataEmerald` false)
  (`self.EnablePermataRuby` false)
  (if (`self.isDeckCardFull`)
    (`self.EnableKartuPedagang` true true)
    (else
      (`self.EnableKartuPedagang` true true true))))

(event `EnablePermataPlayer`
  (`self.EnablePermataSapphire` true true)
  (`self.EnablePermataEmerald` true true)
  (`self.EnablePermataRuby` true true))

(event `EnablePermata`
  (params (`enable?` :type Boolean) (permata :type "/Game/Blueprint/S_Permata Structure"))
  (bind (_sapphire _emerald _ruby) (break `/Game/Blueprint/S_Permata` permata))
  (if `enable?`
    (`|ExecutionSequence`
      (:`then_0`
        (if (> _sapphire 0)
          (`self.EnablePermataSapphire` true true true)
          (else
            (`self.EnablePermataSapphire` true true))))
      (:`then_1`
        (if (> _emerald 0)
          (`self.EnablePermataEmerald` true true true)
          (else
            (`self.EnablePermataEmerald` true true))))
      (:`then_2`
        (if (> _ruby 0)
          (`self.EnablePermataRuby` true true true)
          (else
            (`self.EnablePermataRuby` true true)))))
    (else
      (`|ExecutionSequence`
        (:`then_0`
          (`self.EnablePermataSapphire` false))
        (:`then_1`
          (`self.EnablePermataEmerald` false))
        (:`then_2`
          (`self.EnablePermataRuby` false))))))

(event `DisablePermata`
  (`self.EnablePermataSapphire` false)
  (`self.EnablePermataEmerald` false)
  (`self.EnablePermataRuby` false))

(event `DeckCardFull`)

(event `OnPlayerMoves`
  (params (Move :type String))
  (if (== Move "BeliKartuPedagang")
    (`KismetSystemLibrary.PrintString` "MASUK ON PLAYER MOVES")
    (`self.EnableKartuPedagang` true true)
    (elif (== Move "BeliPermata")
      _
      (elif (== Move "TukarPermata")
        _
        (elif (== Move "UpgradePermata")
          _)))))

(fn `UserConstructionScript`)