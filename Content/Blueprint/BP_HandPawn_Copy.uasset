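; VR hand-tracking player pawn for a networked card and gem (permata) game, seated by authority and local control.
; It spawns attached left and right hands, shows recognised gestures on widgets, and has debug keys to record or delete gestures.
; Grab and release of one to three items relay through Server then Clients events to pickup/drop messages.
; The gem deck follows camera rotation without pitch; card-type actions and slot overlaps are empty stubs.
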(event `self.ReceiveBeginPlay`
  (bind _returnvalue (`KismetMathLibrary.MakeTransform` (0.0 0.0 0.0)))
  (`|ExecutionSequence`
    (:`then_0`
      (`HeadMountedDisplayFunctionLibrary.SetTrackingOrigin` "Floor")
      (`|ExecutionSequence`
        (:`then_0`
          (bind _returnvalue_2 (`|SpawnActorFromClass` "/Game/Blueprint/BP_HandLeft.BP_HandLeft_C" _returnvalue "Undefined" "OverrideRootScale" self "Left" null))
          (bind _output_get (set `self.LeftHand` _returnvalue_2))
          (`self.K2_AttachToActor` _output_get self "None" "SnapToTarget" "SnapToTarget" "KeepWorld" false))
        (:`then_1`
          (bind _returnvalue_3 (`|SpawnActorFromClass` "/Game/Blueprint/BP_HandRight.BP_HandRight_C" _returnvalue "Undefined" "OverrideRootScale" self "Right" null))
          (bind _output_get_2 (set `self.RightHand` _returnvalue_3))
          (`self.K2_AttachToActor` _output_get_2 self "None" "SnapToTarget" "SnapToTarget" "KeepWorld" false))))
    (:`then_1`
      (`|ExecutionSequence`
        (:`then_0`
          (add `/Game/Blueprint/BP_HandLeft.onGestureRecognised` (`self.LeftHand`) (`|CreateDelegate` :!event `GestureRecognisedLeft`))
          (add `/Game/Blueprint/BP_HandLeft.onGestureRecognised` (`self.RightHand`) (`|CreateDelegate` :!event `GestureRecognisedRight`)))
        (:`then_1`
          (bind _aswb_cur_gesture (cast `/Game/Blueprint/WB_CurGesture` (`WidgetComponent.GetUserWidgetObject` (`self.Widget Left`))))
          (set `self.As WB Cur Gesture Left` _aswb_cur_gesture)
          (bind _aswb_cur_gesture_2 (cast `/Game/Blueprint/WB_CurGesture` (`WidgetComponent.GetUserWidgetObject` (`self.Widget Right`))))
          (set `self.As WB Cur Gesture Right` _aswb_cur_gesture_2))
        (:`then_2`
          (`/Engine/EditorBlueprintResources/ActorMacros.Switch Has Authority`
            (:`Authority`
              (if (`self.IsLocallyControlled`)
                (`self.K2_SetActorLocationAndRotation` (30.0 90.0 100.0) (struct :`Yaw` 270.0))
                (else
                  (`self.K2_SetActorLocationAndRotation` (-30.0 90.0 100.0) (struct :`Yaw` 270.0)))))))
        (:`then_3`
          (`self.AddWidgetonClient`))))))

(event `Key|C`
  (params (Key :type "Key Structure"))
  (:`Pressed`
    (bind _asbp_game_state_base (cast `/Game/Blueprint/BP_GameStateBase` (`GameplayStatics.GetGameState`)))
    (for _array_element (`/Game/Blueprint/BP_GameStateBase.idPoinTemp` _asbp_game_state_base)
      (`KismetSystemLibrary.PrintString` (`KismetStringLibrary.Conv_IntToString` _array_element)))))

(event `GestureRecognisedLeft`
  (params (GestureName :type String))
  (set `/Game/Blueprint/WB_CurGesture.CurrentGesture` GestureName (`self.As WB Cur Gesture Left`)))

(event `GestureRecognisedRight`
  (params (GestureName :type String))
  (set `/Game/Blueprint/WB_CurGesture.CurrentGesture` GestureName (`self.As WB Cur Gesture Right`)))

(event `OnGrab1`
  (params (AttachedTo1 :type "Actor Object Reference") (LeftHand :type Boolean))
  ;[1 0.9836 0.5086] Grab 1 Permata
  (`self.OnGrab1Server` AttachedTo1 LeftHand))

(event `OnGrab2`
  (params (AttachedTo1 :type "Actor Object Reference") (AttachedTo2 :type "Actor Object Reference") (LeftHand :type Boolean))
  ;[1 0.5616 0.3172] Grab 2 Permata
  (`self.OnGrab2Server` AttachedTo1 AttachedTo2 LeftHand))

(event `OnGrab3`
  (params (AttachedTo1 :type "Actor Object Reference") (AttachedTo2 :type "Actor Object Reference") (AttachedTo3 :type "Actor Object Reference") (LeftHand :type Boolean))
  ;[0.6521 1 0.3638] Grab 3 permata
  (`self.OnGrab3Server` AttachedTo1 AttachedTo2 AttachedTo3 LeftHand))

(event `OnGrab2Server`
  (params (AttachedTo1 :type "Actor Object Reference") (AttachedTo2 :type "Actor Object Reference") (LeftHand :type Boolean))
  ;[1 0.5616 0.3172] Grab 2 Permata
  (`self.OnGrab2Clients` AttachedTo1 AttachedTo2 LeftHand))

(event `OnGrab1Server`
  (params (AttachedTo1 :type "Actor Object Reference") (LeftHand :type Boolean))
  ;[1 0.9836 0.5086] Grab 1 Permata
  (`self.OnGrab1Clients` AttachedTo1 LeftHand))

(event `OnGrab3Server`
  (params (AttachedTo1 :type "Actor Object Reference") (AttachedTo2 :type "Actor Object Reference") (AttachedTo3 :type "Actor Object Reference") (LeftHand :type Boolean))
  ;[0.6521 1 0.3638] Grab 3 permata
  (`self.OnGrab3Clients` AttachedTo1 AttachedTo2 AttachedTo3 LeftHand))

(event `Key|R`
  (params (Key :type "Key Structure"))
  (:`Pressed`
    (`/Game/Blueprint/BPC_Hand.RecordGesture` (`/Game/Blueprint/BP_HandLeft.OculusHand` (`self.RightHand`)) (`self.GestureNameRecord`))
    (`KismetSystemLibrary.PrintString` "Recoreded Right")))

(event `OnGrab1Clients`
  (params (AttachedTo1 :type "Actor Object Reference") (LeftHand :type Boolean))
  ;[1 0.9836 0.5086] Grab 1 Permata
  (if LeftHand
    (message `/Game/Blueprint/PickupActorInterface.Pickup` AttachedTo1 (`/Game/Blueprint/BP_HandLeft.OculusHand` (`self.LeftHand`)))
    (else
      (message `/Game/Blueprint/PickupActorInterface.Pickup` AttachedTo1 (`/Game/Blueprint/BP_HandLeft.OculusHand` (`self.RightHand`))))))

(event `OnGrab2Clients`
  (params (AttachedTo1 :type "Actor Object Reference") (AttachedTo2 :type "Actor Object Reference") (LeftHand :type Boolean))
  ;[1 0.5616 0.3172] Grab 2 Permata
  (if LeftHand
    (message `/Game/Blueprint/PickupActorInterface.Pickup` AttachedTo1 (`/Game/Blueprint/BP_HandLeft.OculusHand` (`self.LeftHand`)))
    (message `/Game/Blueprint/PickupActorInterface.Pickup` AttachedTo2 (`/Game/Blueprint/BP_HandLeft.OculusHand` (`self.LeftHand`)))
    (else
      (message `/Game/Blueprint/PickupActorInterface.Pickup` AttachedTo1 (`/Game/Blueprint/BP_HandLeft.OculusHand` (`self.RightHand`)))
      (message `/Game/Blueprint/PickupActorInterface.Pickup` AttachedTo2 (`/Game/Blueprint/BP_HandLeft.OculusHand` (`self.RightHand`))))))

(event `OnGrab3Clients`
  (params (AttachedTo1 :type "Actor Object Reference") (AttachedTo2 :type "Actor Object Reference") (AttachedTo3 :type "Actor Object Reference") (LeftHand :type Boolean))
  ;[0.6521 1 0.3638] Grab 3 permata
  (if LeftHand
    (message `/Game/Blueprint/PickupActorInterface.Pickup` AttachedTo1 (`/Game/Blueprint/BP_HandLeft.OculusHand` (`self.LeftHand`)))
    (message `/Game/Blueprint/PickupActorInterface.Pickup` AttachedTo2 (`/Game/Blueprint/BP_HandLeft.OculusHand` (`self.LeftHand`)))
    (message `/Game/Blueprint/PickupActorInterface.Pickup` AttachedTo3 (`/Game/Blueprint/BP_HandLeft.OculusHand` (`self.LeftHand`)))
    (else
      (message `/Game/Blueprint/PickupActorInterface.Pickup` AttachedTo1 (`/Game/Blueprint/BP_HandLeft.OculusHand` (`self.RightHand`)))
      (message `/Game/Blueprint/PickupActorInterface.Pickup` AttachedTo2 (`/Game/Blueprint/BP_HandLeft.OculusHand` (`self.RightHand`)))
      (message `/Game/Blueprint/PickupActorInterface.Pickup` AttachedTo3 (`/Game/Blueprint/BP_HandLeft.OculusHand` (`self.RightHand`))))))

(event `Key|L`
  (params (Key :type "Key Structure"))
  (:`Pressed`
    (`/Game/Blueprint/BPC_Hand.RecordGesture` (`/Game/Blueprint/BP_HandLeft.OculusHand` (`self.LeftHand`)) (`self.GestureNameRecord`))
    (`KismetSystemLibrary.PrintString` "Recoreded Left")))

(event `Key|D`
  (params (Key :type "Key Structure"))
  (:`Pressed`
    (`/Game/Blueprint/BPC_Hand.DeleteGesture` (`/Game/Blueprint/BP_HandLeft.OculusHand` (`self.LeftHand`)) (`self.GestureNameRecord`))
    (`/Game/Blueprint/BPC_Hand.DeleteGesture` (`/Game/Blueprint/BP_HandLeft.OculusHand` (`self.RightHand`)) (`self.GestureNameRecord`))
    (`KismetSystemLibrary.PrintString` "Delete Gesture")))

(event `onRelease2`
  (params (Item1 :type "Actor Object Reference") (Item2 :type "Actor Object Reference"))
  ;[1 0.6949 0.2601] Release 2 Item
  (`self.onRelease2Server` Item1 Item2))

(event `onRelease3`
  (params (Item1 :type "Actor Object Reference") (Item2 :type "Actor Object Reference") (Item3 :type "Actor Object Reference"))
  ;[0.5576 1 0.315] Release 3 Item
  (`self.onRelease3Server` Item1 Item2 Item3))

(event `onRelase1`
  (params (Item1 :type "Actor Object Reference"))
  ;[0.9969 1 0.5568] Release 1 Item
  (`self.onRelease1Server` Item1))

(event `self.ReceiveTick`
  (params (DeltaSeconds :type "Float (single-precision)"))
  (bind (_returnvalue_roll _returnvalue_pitch _returnvalue_yaw) (`KismetMathLibrary.BreakRotator` (`SceneComponent.K2_GetComponentRotation` (`self.Camera`))))
  (`SceneComponent.K2_SetWorldRotation` (`self.Deck Permata Mesh`) (`KismetMathLibrary.MakeRotator` _returnvalue_roll 0.0 _returnvalue_yaw) false false))

(event `onRelease1Server`
  (params (Item1 :type "Actor Object Reference"))
  ;[0.9969 1 0.5568] Release 1 Item
  (`self.onRelease1Clients` Item1))

(event `onRelease2Server`
  (params (Item1 :type "Actor Object Reference") (Item2 :type "Actor Object Reference"))
  ;[1 0.6949 0.2601] Release 2 Item
  (`self.onRelease2Clients` Item1 Item2))

(event `onRelease3Server`
  (params (Item1 :type "Actor Object Reference") (Item2 :type "Actor Object Reference") (Item3 :type "Actor Object Reference"))
  ;[0.5576 1 0.315] Release 3 Item
  (`self.onRelease3Clients` Item1 Item2 Item3))

(event `onRelease2Clients`
  (params (Item1 :type "Actor Object Reference") (Item2 :type "Actor Object Reference"))
  ;[1 0.6949 0.2601] Release 2 Item
  (message `/Game/Blueprint/PickupActorInterface.Drop` Item1)
  (message `/Game/Blueprint/PickupActorInterface.Drop` Item2))

(event `onRelease1Clients`
  (params (Item1 :type "Actor Object Reference"))
  ;[0.9969 1 0.5568] Release 1 Item
  (message `/Game/Blueprint/PickupActorInterface.Drop` Item1))

(event `onRelease3Clients`
  (params (Item1 :type "Actor Object Reference") (Item2 :type "Actor Object Reference") (Item3 :type "Actor Object Reference"))
  ;[0.5576 1 0.315] Release 3 Item
  (message `/Game/Blueprint/PickupActorInterface.Drop` Item1)
  (message `/Game/Blueprint/PickupActorInterface.Drop` Item2)
  (message `/Game/Blueprint/PickupActorInterface.Drop` Item3))

(event `self.kartu1.OnComponentBeginOverlap`
  (params (OverlappedComponent :type "PrimitiveComponent Object Reference") (OtherActor :type "Actor Object Reference") (OtherComp :type "PrimitiveComponent Object Reference") (OtherBodyIndex :type Integer) (bFromSweep :type Boolean) (SweepResult :type "HitResult Structure (by ref)"))
  (if (`self.ActorHasTag` OtherActor "kartuPedagang")
    _))

(event `self.kartu2.OnComponentBeginOverlap`
  (params (OverlappedComponent :type "PrimitiveComponent Object Reference") (OtherActor :type "Actor Object Reference") (OtherComp :type "PrimitiveComponent Object Reference") (OtherBodyIndex :type Integer) (bFromSweep :type Boolean) (SweepResult :type "HitResult Structure (by ref)"))
  (if (`self.ActorHasTag` OtherActor "kartuPedagang")
    _))

(event `self.kartu3.OnComponentBeginOverlap`
  (params (OverlappedComponent :type "PrimitiveComponent Object Reference") (OtherActor :type "Actor Object Reference") (OtherComp :type "PrimitiveComponent Object Reference") (OtherBodyIndex :type Integer) (bFromSweep :type Boolean) (SweepResult :type "HitResult Structure (by ref)"))
  (if (`self.ActorHasTag` OtherActor "kartuPedagang")
    _))

(event `self.kartu4.OnComponentBeginOverlap`
  (params (OverlappedComponent :type "PrimitiveComponent Object Reference") (OtherActor :type "Actor Object Reference") (OtherComp :type "PrimitiveComponent Object Reference") (OtherBodyIndex :type Integer) (bFromSweep :type Boolean) (SweepResult :type "HitResult Structure (by ref)"))
  (if (`self.ActorHasTag` OtherActor "kartuPedagang")
    _))

(event `self.TempatMainKartu.OnComponentBeginOverlap`
  (params (OverlappedComponent :type "PrimitiveComponent Object Reference") (OtherActor :type "Actor Object Reference") (OtherComp :type "PrimitiveComponent Object Reference") (OtherBodyIndex :type Integer) (bFromSweep :type Boolean) (SweepResult :type "HitResult Structure (by ref)"))
  (if (`self.ActorHasTag` OtherActor "kartuPedagang")
    (bind _asbp_kartu_pedagang (cast `/Game/Blueprint/Game/BP_KartuPedagang` OtherActor))
    (bind (_id _type) (break `/Game/Blueprint/S_KartuPedagang` (`|GetArrayItem` (`/Game/Blueprint/Game/BP_KartuPedagang.SKartuPedagang` _asbp_kartu_pedagang) (`/Game/Blueprint/Game/BP_KartuPedagang.CardId` _asbp_kartu_pedagang))))
    (if (== _type "beli")
      (`self.BeliPermata`)
      (elif (== _type "tukar")
        (`self.TukarPermata`)
        (elif (== "" "upgrade")
          (`self.UpgradePermata`))))))

(event `self.BoxAtas1.OnComponentBeginOverlap`
  (params (OverlappedComponent :type "PrimitiveComponent Object Reference") (OtherActor :type "Actor Object Reference") (OtherComp :type "PrimitiveComponent Object Reference") (OtherBodyIndex :type Integer) (bFromSweep :type Boolean) (SweepResult :type "HitResult Structure (by ref)"))
  (if (`self.ActorHasTag` OtherActor "permata")
    _))

(event `self.BoxAtas2.OnComponentBeginOverlap`
  (params (OverlappedComponent :type "PrimitiveComponent Object Reference") (OtherActor :type "Actor Object Reference") (OtherComp :type "PrimitiveComponent Object Reference") (OtherBodyIndex :type Integer) (bFromSweep :type Boolean) (SweepResult :type "HitResult Structure (by ref)"))
  (if (`self.ActorHasTag` OtherActor "permata")
    _))

(event `self.BoxAtas3.OnComponentBeginOverlap`
  (params (OverlappedComponent :type "PrimitiveComponent Object Reference") (OtherActor :type "Actor Object Reference") (OtherComp :type "PrimitiveComponent Object Reference") (OtherBodyIndex :type Integer) (bFromSweep :type Boolean) (SweepResult :type "HitResult Structure (by ref)"))
  (if (`self.ActorHasTag` OtherActor "permata")
    _))

(event `self.BoxAtas4.OnComponentBeginOverlap`
  (params (OverlappedComponent :type "PrimitiveComponent Object Reference") (OtherActor :type "Actor Object Reference") (OtherComp :type "PrimitiveComponent Object Reference") (OtherBodyIndex :type Integer) (bFromSweep :type Boolean) (SweepResult :type "HitResult Structure (by ref)"))
  (if (`self.ActorHasTag` OtherActor "permata")
    _))

(event `self.BoxAtas5.OnComponentBeginOverlap`
  (params (OverlappedComponent :type "PrimitiveComponent Object Reference") (OtherActor :type "Actor Object Reference") (OtherComp :type "PrimitiveComponent Object Reference") (OtherBodyIndex :type Integer) (bFromSweep :type Boolean) (SweepResult :type "HitResult Structure (by ref)"))
  (if (`self.ActorHasTag` OtherActor "permata")
    _))

(event `self.BoxBawah1.OnComponentBeginOverlap`
  (params (OverlappedComponent :type "PrimitiveComponent Object Reference") (OtherActor :type "Actor Object Reference") (OtherComp :type "PrimitiveComponent Object Reference") (OtherBodyIndex :type Integer) (bFromSweep :type Boolean) (SweepResult :type "HitResult Structure (by ref)"))
  (if (`self.ActorHasTag` OtherActor "permata")
    _))

(event `self.BoxBawah2.OnComponentBeginOverlap`
  (params (OverlappedComponent :type "PrimitiveComponent Object Reference") (OtherActor :type "Actor Object Reference") (OtherComp :type "PrimitiveComponent Object Reference") (OtherBodyIndex :type Integer) (bFromSweep :type Boolean) (SweepResult :type "HitResult Structure (by ref)"))
  (if (`self.ActorHasTag` OtherActor "permata")
    _))

(event `self.BoxBawah3.OnComponentBeginOverlap`
  (params (OverlappedComponent :type "PrimitiveComponent Object Reference") (OtherActor :type "Actor Object Reference") (OtherComp :type "PrimitiveComponent Object Reference") (OtherBodyIndex :type Integer) (bFromSweep :type Boolean) (SweepResult :type "HitResult Structure (by ref)"))
  (if (`self.ActorHasTag` OtherActor "permata")
    _))

(event `self.BoxBawah4.OnComponentBeginOverlap`
  (params (OverlappedComponent :type "PrimitiveComponent Object Reference") (OtherActor :type "Actor Object Reference") (OtherComp :type "PrimitiveComponent Object Reference") (OtherBodyIndex :type Integer) (bFromSweep :type Boolean) (SweepResult :type "HitResult Structure (by ref)"))
  (if (`self.ActorHasTag` OtherActor "permata")
    _))

(event `self.BoxBawah5.OnComponentBeginOverlap`
  (params (OverlappedComponent :type "PrimitiveComponent Object Reference") (OtherActor :type "Actor Object Reference") (OtherComp :type "PrimitiveComponent Object Reference") (OtherBodyIndex :type Integer) (bFromSweep :type Boolean) (SweepResult :type "HitResult Structure (by ref)"))
  (if (`self.ActorHasTag` OtherActor "permata")
    _))

(event `AddWidgetonClient`
  (bind _returnvalue (`|CreateWidget` "/Game/Blueprint/WB_Rounds.WB_Rounds_C"))
  (bind _output_get (set `self.WBGamaplay` _returnvalue))
  (`UserWidget.AddToViewport` _output_get 0))

(event `BeliKartuPoin`
  (params (Kondisi :type Boolean) (point :type Integer))
  (if Kondisi
    (bind _asbp_player_state (cast `/Game/Blueprint/BP_PlayerState` (`self.PlayerState`)))
    (set `/Game/Blueprint/BP_PlayerState.point` point _asbp_player_state)))

(event `BeliPermata`)

(event `TukarPermata`)

(event `UpgradePermata`)

(fn `UserConstructionScript`
  (set `self.DeckKartu` (`|MakeArray` (`self.kartu1`) (`self.kartu2`) (`self.kartu3`) (`self.kartu4`)))
  (set `self.DeckPermata` (`|MakeArray` (`self.BoxAtas1`) (`self.BoxAtas2`) (`self.BoxAtas3`) (`self.BoxAtas4`) (`self.BoxAtas5`) (`self.BoxBawah1`) (`self.BoxBawah2`) (`self.BoxBawah3`) (`self.BoxBawah4`) (`self.BoxBawah5`))))