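; BP_PickupCube is a physics cube that BP_MotionController can pick up and drop.
; Pickup disables physics and attaches the cube to the given component, optionally snapping to a socket, and first calls CallPickup on its PickupObject component if already grabbed.
; Drop detaches it and restores physics.
; Getters expose that component and a separate pose animation for each hand.
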(event `self.ReceiveBeginPlay`
  (`PrimitiveComponent.SetEnableGravity` (`self.StaticMeshComponent`) true))

(event `/Game/Blueprint/PickupActorInterface.Pickup`
  (params (AttachTo :type "SceneComponent Object Reference"))
  (bind _returnvalue (select `bool` (`self.bSnapToSocket?`) :`false` "KeepWorld" :`true` "SnapToTarget" :!type "EAttachmentRule Enum"))
  (if (not (not (`self.bGrabbed?`)))
    (`/Game/Blueprint/BPC_PickupObject.Pickup` (`self.PickupObject`) AttachTo))
  (`PrimitiveComponent.SetSimulatePhysics` (`self.StaticMeshComponent`) false)
  (`SceneComponent.K2_AttachToComponent` (`self.RootComponent`) AttachTo (select `bool` (`self.bSnapToSocket?`) :`true` (`self.SnapSocket`)) _returnvalue _returnvalue "KeepWorld" false)
  (set `self.bGrabbed?` true))

(event `/Game/Blueprint/PickupActorInterface.Drop`
  (`PrimitiveComponent.SetSimulatePhysics` (`self.StaticMeshComponent`) true)
  (`self.K2_DetachFromActor` "KeepWorld" "KeepWorld" "KeepWorld")
  (set `self.bGrabbed?` false))

(fn `GetAnimSequence`
  (params (Hand :type "EControllerHand Enum" :default "Left"))
  (returns (AnimSequence :type "AnimSequence Object Reference"))
  (switch `EControllerHand` Hand
    (:`Left`
      (return (`self.LeftHandPose`)))
    (:`Right`
      (return (`self.RightHandPose`)))))

(fn `GetPickupComponent`
  (returns (PickupComponent :type "/Game/Blueprint/BPC_PickupObject Object Reference"))
  (return (`self.PickupObject`)))

(fn `UserConstructionScript`)