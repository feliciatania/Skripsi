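; VR pawn that recognizes hand gestures on both hands and shows the current gesture name through a widget.
; Both hands' recognition events feed a handler that writes the name to WB_CurGesture; its per-gesture switch branches are empty and the Hand action calls are unwired.
; BeginPlay sets floor tracking and, if the widget's render target is valid, composites it onto the spectator screen.
; R, L and D keys record or delete gestures for authoring.
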(event `self.ReceiveBeginPlay`
  (bind _returnvalue (`WidgetComponent.GetRenderTarget` (`self.Widget`)))
  (`|ExecutionSequence`
    (:`then_0`
      (`HeadMountedDisplayFunctionLibrary.SetTrackingOrigin` "Floor")
      (add `/Game/Blueprint/BPC_OculusHandGesture.OnGestureRecognised` (`self.LeftHand`) (`|CreateDelegate` :!event `GestureRecognised`))
      (add `/Game/Blueprint/BPC_OculusHandGesture.OnGestureRecognised` (`self.RightHand`) (`|CreateDelegate` :!event `GestureRecognised`))
      (bind _aswb_cur_gesture (cast `/Game/Blueprint/WB_CurGesture` (`WidgetComponent.GetUserWidgetObject` (`self.Widget`))))
      (set `self.As WB Cur Gesture` _aswb_cur_gesture))
    (:`then_1`
      (`/Engine/EditorBlueprintResources/StandardMacros.IsValid` _returnvalue
        (:`Is Valid`
          (`/Engine/EditorBlueprintResources/StandardMacros.DoOnce` false
            (:`Completed`
              (`HeadMountedDisplayFunctionLibrary.SetSpectatorScreenMode` "TexturePlusEye")
              (`HeadMountedDisplayFunctionLibrary.SetSpectatorScreenTexture` _returnvalue)
              (`HeadMountedDisplayFunctionLibrary.SetSpectatorScreenModeTexturePlusEyeLayout` (0.0 0.0) (1.0 1.0) (0.0 0.0) (1.0 1.0) true true true))))
        (:`Is Not Valid`
          (`KismetSystemLibrary.Delay` 0.2))))))

(event `GestureRecognised`
  (params (GestureName :type String))
  (switch `string` GestureName
    (:`Default`
      _)
    (:`Idle`
      _)
    (:`Grab1`
      _)
    (:`Grab2`
      _)
    (:`Grab3`
      _)
    (:`GrabKartu`
      _)
    (:`Teleport`
      _))
  (set `/Game/Blueprint/WB_CurGesture.CurrentGesture` GestureName (`self.As WB Cur Gesture`)))

(event `Key|R`
  (params (Key :type "Key Structure"))
  (:`Pressed`
    (`/Game/Blueprint/BPC_OculusHandGesture.RecordGesture` (`self.RightHand`) (`self.GestrureName`))
    (`KismetSystemLibrary.PrintString` "Recoreded Right")))

(event `Key|L`
  (params (Key :type "Key Structure"))
  (:`Pressed`
    (`/Game/Blueprint/BPC_OculusHandGesture.RecordGesture` (`self.LeftHand`) (`self.GestrureName`))
    (`KismetSystemLibrary.PrintString` "Recoreded Left")))

(event `Key|D`
  (params (Key :type "Key Structure"))
  (:`Pressed`
    (`/Game/Blueprint/BPC_OculusHandGesture.DeleteGesture` (`self.RightHand`) (`self.GestrureName`))
    (`/Game/Blueprint/BPC_OculusHandGesture.DeleteGesture` (`self.LeftHand`) (`self.GestrureName`))
    (`KismetSystemLibrary.PrintString` "Delete Gesture")))

(fn `UserConstructionScript`)