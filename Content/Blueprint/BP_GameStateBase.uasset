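; Game state for a turn-based card game with point (Poin) and merchant (Pedagang) cards, managing dealing, turns and rounds.
; On play it caches slot locations from BP_CollisonBoxKartu actors, then the authority shuffles IDs and spawns opening cards, reshuffling merchants until enough low-ID cards lead.
; Spawn events refill slots from the shuffled lists.
; Turns alternate between Server and Client, or stay solo, advancing rounds until MaxRound triggers game over.
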(event `self.ReceiveBeginPlay`
  (`self.PlayGame`))

(event `PlayGame`
  (bind _outactors (`GameplayStatics.GetAllActorsOfClass` "/Game/Blueprint/BP_CollisonBoxKartu.BP_CollisonBoxKartu_C"))
  (for _array_element _outactors
    (if (`/Game/Blueprint/BP_CollisonBoxKartu.isPointCard` _array_element)
      (bind _id (`/Game/Blueprint/BP_CollisonBoxKartu.id` _array_element))
      (bind _returnvalue (`SceneComponent.K2_GetComponentLocation` (`/Game/Blueprint/BP_CollisonBoxKartu.DefaultSceneRoot` _array_element)))
      (`KismetArrayLibrary.Array_Set` (`self.TriggerPoinLoc`) _id _returnvalue)
      (else
        (`KismetArrayLibrary.Array_Set` (`self.TriggerPedagangLoc`) _id _returnvalue))))
  (`self.ShuffleKartu`)
  (`self.StartRound`))

(event `ShuffleKartu`
  (set `self.countPoin` 5)
  (set `self.countPedagang` 5)
  (`self.ShuffleKartuPoin`)
  (`self.ShuffleKartuPedagang`))

(event `ShuffleKartuPoin`
  (`/Engine/EditorBlueprintResources/ActorMacros.Switch Has Authority`
    (:`Authority`
      (bind _output_get (set `self.idPoinTemp` (`self.idPoin`)))
      (`KismetArrayLibrary.Array_Shuffle` _output_get)
      (for _index (range (`self.countPoin`))
        (bind _returnvalue (`|SpawnActorFromClass` "/Game/Blueprint/Game/BP_KartuPoin.BP_KartuPoin_C" (`KismetMathLibrary.MakeTransform` (`|GetArrayItem` (`self.TriggerPoinLoc`) _index)) "Undefined" "OverrideRootScale" null null))
        (`/Game/Blueprint/Game/BP_KartuPoin.setKartu` _returnvalue (`|GetArrayItem` (`self.idPoinTemp`) _index))))))

(event `ShuffleKartuPedagang`
  (`/Engine/EditorBlueprintResources/ActorMacros.Switch Has Authority`
    (:`Authority`
      (bind _output_get (set `self.idPedagangTemp` (`self.idPedagang`)))
      (`KismetArrayLibrary.Array_Shuffle` _output_get)
      (bind _condition (`self.CheckShuffleKartuPedagang`))
      (if _condition
        (for _index (range (`self.countPedagang`))
          (bind _returnvalue (`|SpawnActorFromClass` "/Game/Blueprint/Game/BP_KartuPedagang.BP_KartuPedagang_C" (`KismetMathLibrary.MakeTransform` (`|GetArrayItem` (`self.TriggerPedagangLoc`) _index)) "Undefined" "OverrideRootScale" null null))
          (`/Game/Blueprint/Game/BP_KartuPedagang.setKartu` _returnvalue (`|GetArrayItem` (`self.idPedagangTemp`) _index)))))))

(event `SpawnKartuPoin`
  (params (Triggerid :type Integer))
  (if (<= (`self.countPoin`) 10)
    (bind _result (`/Engine/EditorBlueprintResources/StandardMacros.IncrementInt` (`self.countPoin`))
      (:`  `
        (bind _returnvalue (`|SpawnActorFromClass` "/Game/Blueprint/Game/BP_KartuPoin.BP_KartuPoin_C" (`KismetMathLibrary.MakeTransform` (`|GetArrayItem` (`self.TriggerPoinLoc`) Triggerid)) "Undefined" "OverrideRootScale" null null))
        (`/Game/Blueprint/Game/BP_KartuPoin.setKartu` _returnvalue (`|GetArrayItem` (`self.idPoinTemp`) _result))))))

(event `SpawnKartuPedagang`
  (params (Triggerid :type Integer))
  (if (<= (`self.countPedagang`) 19)
    (bind _result (`/Engine/EditorBlueprintResources/StandardMacros.IncrementInt` (`self.countPedagang`))
      (:`  `
        (bind _returnvalue (`|SpawnActorFromClass` "/Game/Blueprint/Game/BP_KartuPedagang.BP_KartuPedagang_C" (`KismetMathLibrary.MakeTransform` (`|GetArrayItem` (`self.TriggerPedagangLoc`) Triggerid)) "Undefined" "OverrideRootScale" null null))
        (`/Game/Blueprint/Game/BP_KartuPedagang.setKartu` _returnvalue (`|GetArrayItem` (`self.idPedagangTemp`) _result))))))

(event `NextGiliranPlayer`
  (if (`self.isGameOver`)
    _
    (elif (== (`self.playerCount`) 1)
      (set `self.CurrentTurn` "NewEnumerator0")
      (`self.NextRound` :!label _label)
      (if (not (`self.isGameOver`))
        (`self.onPlayerTurnStart` (`self.CurrentTurn`)))
      (else
        (switch `/Game/Blueprint/E_Turn` (`self.CurrentTurn`)
          (:`NewEnumerator0`
            (set `self.CurrentTurn` "NewEnumerator1"))
          (:`NewEnumerator1`
            (set `self.CurrentTurn` "NewEnumerator0")))
        (bind _result (`/Engine/EditorBlueprintResources/StandardMacros.IncrementInt` (`self.CounterGiliran`))
          (:`  `
            (if (> _result 2)
              (goto _label))))))))

(event `StartRound`
  (`/Engine/EditorBlueprintResources/ActorMacros.Switch Has Authority`
    (:`Authority`
      (bind _output_get (set `self.playerCount` (`GameplayStatics.GetNumPlayerControllers`)))
      (set `self.Rounds` 1)
      (if (== _output_get 1)
        (bind _output_get_2 (set `self.CurrentTurn` "NewEnumerator0"))
        (`KismetSystemLibrary.Delay` 1.0)
        (`self.onPlayerTurnStart` _output_get_2)
        (else
          (bind _output_get_3 (set `self.CurrentTurn` (select `bool` (`KismetMathLibrary.RandomBool`) :`false` "NewEnumerator0" :`true` "NewEnumerator1" :!type "/Game/Blueprint/E_Turn Enum")))
          (`KismetSystemLibrary.Delay` 1.0)
          (`self.onPlayerTurnStart` _output_get_3))))))

(event `NextRound`
  (if (< (`self.Rounds`) (`self.MaxRound`))
    (set `self.Rounds` (+ (`self.Rounds`) 1))
    (set `self.CounterGiliran` 1)
    (else
      (set `self.isGameOver` true)
      (`self.onGameOver`)
      (`KismetSystemLibrary.PrintString` "GAMEOVERrrrrrrrrrrrrrrrrrrrrrrr"))))

(fn `CheckShuffleKartuPedagang`
  (returns (condition :type Boolean))
  (locals (whileCondition :type Boolean) (CountKartuBeli :type Integer))
  (bind _output_get (set `self.idPedagangTemp` (`self.idPedagang`)))
  (`KismetArrayLibrary.Array_Shuffle` _output_get)
  (for _index (range 6)
    (if (<= (`|GetArrayItem` (`self.idPedagangTemp`) _index) 6)
      (`/Engine/EditorBlueprintResources/StandardMacros.IncrementInt` (`local.CountKartuBeli`))))
  (while (< (`local.CountKartuBeli`) (`self.playerCount`))
    (`KismetArrayLibrary.Array_Shuffle` (`self.idPedagangTemp`))
    (set `local.CountKartuBeli` 0)
    (for _index_2 (range 6)
      (if (<= (`|GetArrayItem` (`self.idPedagangTemp`) _index_2) 6)
        (`/Engine/EditorBlueprintResources/StandardMacros.IncrementInt` (`local.CountKartuBeli`)))))
  (return true))

(fn `SetTriggerLocation`
  (locals (SpawnKartuLoc :type "Array of /Game/Blueprint/BP_CollisonBoxKartu Object Reference"))
  (bind _outactors (`GameplayStatics.GetAllActorsOfClass` "/Game/Blueprint/BP_CollisonBoxKartu.BP_CollisonBoxKartu_C"))
  (bind _output_get (set `local.SpawnKartuLoc` _outactors))
  (for _array_element _output_get
    (if (`/Game/Blueprint/BP_CollisonBoxKartu.isPointCard` _array_element)
      (bind _id (`/Game/Blueprint/BP_CollisonBoxKartu.id` _array_element))
      (bind _returnvalue (`SceneComponent.K2_GetComponentLocation` (`/Game/Blueprint/BP_CollisonBoxKartu.DefaultSceneRoot` _array_element)))
      (`KismetArrayLibrary.Array_Set` (`self.TriggerPoinLoc`) _id _returnvalue)
      (else
        (`KismetArrayLibrary.Array_Set` (`self.TriggerPedagangLoc`) _id _returnvalue)))
    (return)))

(fn `UserConstructionScript`)