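; VR pawn for the main menu that gives the player two hand menu actors.
; On BeginPlay it sets a floor tracking origin, then spawns and attaches left and right BP_HandMenu actors.
; Left and right menu pinch inputs forward press and release events to the matching hand.
; A SpawnMainMenu spawn using GetMenuTransform is left disconnected, and that function's camera-facing transform is unused.
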(event `self.ReceiveBeginPlay`
  (bind _returnvalue (`KismetMathLibrary.MakeTransform` (0.0 0.0 0.0)))
  (`|ExecutionSequence`
    (:`then_0`
      (`HeadMountedDisplayFunctionLibrary.SetTrackingOrigin` "Floor"))
    (:`then_1`
      (`|ExecutionSequence`
        (:`then_0`
          (bind _returnvalue_2 (`|SpawnActorFromClass` "/Game/Blueprint/MainMenu/BP_HandMenu.BP_HandMenu_C" _returnvalue "AlwaysSpawn" "OverrideRootScale" self "Left" null))
          (bind _output_get (set `self.Left` _returnvalue_2))
          (`self.K2_AttachToActor` _output_get self "None" "SnapToTarget" "SnapToTarget" "KeepWorld" true))
        (:`then_1`
          (bind _returnvalue_3 (`|SpawnActorFromClass` "/Game/Blueprint/MainMenu/BP_HandMenu.BP_HandMenu_C" _returnvalue "AlwaysSpawn" "OverrideRootScale" self "Right" null))
          (bind _output_get_2 (set `self.Right` _returnvalue_3))
          (`self.K2_AttachToActor` _output_get_2 self "None" "SnapToTarget" "SnapToTarget" "KeepWorld" true))))))

(event `self.ReceiveTick`
  (params (DeltaSeconds :type "Float (single-precision)")))

(event `InputAction|LeftMenuPinch`
  (params (Key :type "Key Structure"))
  (bind _left (`self.Left`))
  (:`Pressed`
    (`/Game/Blueprint/MainMenu/BP_HandMenu.PressL` _left))
  (:`Released`
    (`/Game/Blueprint/MainMenu/BP_HandMenu.ReleaseL` _left)))

(event `InputAction|RightMenuPinch`
  (params (Key :type "Key Structure"))
  (bind _right (`self.Right`))
  (:`Pressed`
    (`/Game/Blueprint/MainMenu/BP_HandMenu.PressR` _right))
  (:`Released`
    (`/Game/Blueprint/MainMenu/BP_HandMenu.ReleaseR` _right)))

(fn `UserConstructionScript`)