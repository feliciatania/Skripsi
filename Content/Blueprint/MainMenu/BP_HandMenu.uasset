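; BP_HandMenu is a main menu actor that points at widgets using Oculus hand tracking.
; Each tick, when the selected hand has high tracking confidence and a valid pointer pose, both widget interaction components move to that pose.
; Press and release events all send left-mouse pointer presses; none releases the key.
; Line trace update and collapse functions are empty stubs.
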(event `self.ReceiveBeginPlay`
  (bind _widgetinteractionleft (`self.WidgetInteractionLeft`))
  (switch `EControllerHand` (`self.Hand`)
    (:`Left`
      (set `WidgetInteractionComponent.VirtualUserIndex` 0 _widgetinteractionleft))
    (:`Right`
      (set `WidgetInteractionComponent.VirtualUserIndex` 1 _widgetinteractionleft))))

(event `self.ReceiveTick`
  (params (DeltaSeconds :type "Float (single-precision)"))
  (bind _returnvalue (`self.GetTransform`))
  (bind (_returnvalue_location _returnvalue_rotation) (`KismetMathLibrary.BreakTransform` (`OculusInputFunctionLibrary.GetPointerPose` (`self.GetOculusHand`))))
  (`|ExecutionSequence`
    (:`then_0`
      (switch `ETrackingConfidence` (`OculusInputFunctionLibrary.GetTrackingConfidence` (`self.GetOculusHand`))
        (:`Low`
          (`self.CollapseLineTrace`))
        (:`High`
          (if (`OculusInputFunctionLibrary.IsPointerPoseValid` (`self.GetOculusHand`))
            (`SceneComponent.K2_SetWorldLocationAndRotation` (`self.WidgetInteractionLeft`) (`KismetMathLibrary.TransformLocation` _returnvalue _returnvalue_location) (`KismetMathLibrary.TransformRotation` _returnvalue _returnvalue_rotation) false false)
            (`SceneComponent.K2_SetWorldLocationAndRotation` (`self.WidgetInteractionRight`) (`KismetMathLibrary.TransformLocation` _returnvalue _returnvalue_location) (`KismetMathLibrary.TransformRotation` _returnvalue _returnvalue_rotation) false false)
            (`self.UpdateLineTrace`)
            (if (`GameplayStatics.BreakHitResult` (`WidgetInteractionComponent.GetLastHitResult` (`self.WidgetInteractionLeft`)))
              (`self.UpdateLineTrace`)
              (else
                (`self.CollapseLineTrace`)))
            (else
              (`self.CollapseLineTrace`))))))))

(event `PressL`
  (`WidgetInteractionComponent.PressPointerKey` (`self.WidgetInteractionLeft`) "LeftMouseButton")
  (`KismetSystemLibrary.PrintString` "rightttt"))

(event `ReleaseL`
  (`WidgetInteractionComponent.PressPointerKey` (`self.WidgetInteractionLeft`) "LeftMouseButton"))

(event `PressR`
  (`WidgetInteractionComponent.PressPointerKey` (`self.WidgetInteractionRight`) "LeftMouseButton")
  (`KismetSystemLibrary.PrintString` "leftttt"))

(event `ReleaseR`
  (`WidgetInteractionComponent.PressPointerKey` (`self.WidgetInteractionRight`) "LeftMouseButton"))

(fn `CollapseLineTrace`)

(fn `GetOculusHand`
  (returns (ReturnValue :type "EOculusHandType Enum"))
  (return (select `EControllerHand` (`self.Hand`) :`Left` "HandLeft" :`Right` "HandRight" :!type "EOculusHandType Enum")))

(fn `UpdateLineTrace`)

(fn `UserConstructionScript`)