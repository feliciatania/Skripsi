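; SpawnMainMenu is a Blueprint for the main menu, built around a WidgetMenu component that can be shown or hidden in game.
; Its only working event, SpawnOptionMenu, hides that component and disables its collision.
; BeginPlay and SpawnMainMenu are empty, leaving the creation of main and option menu widgets, UI-only input setup and re-showing logic disconnected.
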(event `self.ReceiveBeginPlay`)

(event `SpawnMainMenu`)

(event `SpawnOptionMenu`
  (bind _widgetmenu (`self.WidgetMenu`))
  (`SceneComponent.SetHiddenInGame` _widgetmenu true false)
  (`PrimitiveComponent.SetCollisionEnabled` _widgetmenu "NoCollision"))

(fn `UserConstructionScript`)