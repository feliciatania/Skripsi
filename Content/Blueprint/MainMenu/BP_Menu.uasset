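; BP_Menu is a main menu Blueprint that switches its Widget component between the menu and options screens.
; SpawnMainMenu and SpawnOption each create a new W_Menu or W_Option and assign it to that component.
; Logic to find these widgets and bind their click delegates is present but unconnected, so nothing in this graph triggers either swap.
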(event `self.ReceiveBeginPlay`)

(event `SpawnOption`
  (bind _returnvalue (`|CreateWidget` "/Game/Blueprint/MainMenu/W_Option.W_Option_C"))
  (`WidgetComponent.SetWidget` (`self.Widget`) _returnvalue))

(event `SpawnMainMenu`
  (bind _returnvalue (`|CreateWidget` "/Game/Blueprint/MainMenu/W_Menu.W_Menu_C"))
  (`WidgetComponent.SetWidget` (`self.Widget`) _returnvalue))

(fn `UserConstructionScript`)