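; BP_permataSapphire is a sapphire gem actor with switchable collision and grab eligibility.
; On BeginPlay it turns off mesh physics and binds an event to the first player's BP_PlayerState for enabling the sapphire.
; Events toggle mesh collision, with World variants gated by CheckHasOwner, whose body is unwired.
; SetCanGrab derives CanGrab from its Enable, HasOwner and World inputs, plus OwnerPawn validity for unowned world gems.
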(event `self.ReceiveBeginPlay`
  (`parent.ReceiveBeginPlay`)
  (`PrimitiveComponent.SetSimulatePhysics` (`self.StaticMeshComponent`) false)
  (bind _asbp_player_state (cast `/Game/Blueprint/BP_PlayerState` (`Pawn.PlayerState` (`GameplayStatics.GetPlayerCharacter` 0))))
  (add `/Game/Blueprint/BP_PlayerState.EnablePermataSapphire` _asbp_player_state (`|CreateDelegate` :!event `SetCanGrab`)))

(event `DisableAllCollision`
  (`PrimitiveComponent.SetCollisionEnabled` (`self.StaticMeshComponent`) "NoCollision"))

(event `EnableAllCollision`
  (`PrimitiveComponent.SetCollisionEnabled` (`self.StaticMeshComponent`) "QueryAndPhysics"))

(event `DisableWorldCollision`
  (if (not (`self.CheckHasOwner`))
    (`PrimitiveComponent.SetCollisionEnabled` (`self.StaticMeshComponent`) "NoCollision")))

(event `EnableWorldCollision`
  (if (not (`self.CheckHasOwner`))
    (`PrimitiveComponent.SetCollisionEnabled` (`self.StaticMeshComponent`) "QueryAndPhysics")))

(event `SetCanGrab`
  (params (enable :type Boolean) (hasOwner :type Boolean) (world :type Boolean))
  (set `self.Has Owner` hasOwner)
  (set `self.World` world)
  (if enable
    (if (`self.Has Owner`)
      (set `self.CanGrab?` true)
      (elif (`self.Has Owner`)
        (`self.ownerPawn`
          (:`then`
            (set `self.CanGrab?` true))
          (:`else`
            (set `self.CanGrab?` false)))
        (elif (`self.World`)
          (`self.ownerPawn`
            (:`then`
              (set `self.CanGrab?` false))
            (:`else`
              (set `self.CanGrab?` true)))
          (else
            (set `self.CanGrab?` false)))))
    (else
      (set `self.CanGrab?` false))))

(fn `UserConstructionScript`
  (`parent.UserConstructionScript`))