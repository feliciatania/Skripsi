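; BP_KartuPedagang is a merchant card actor that can be grabbed and dropped, with a swappable face material.
; Pickup attaches the card to the given component, optionally snapping to a socket, and notifies BPCPickupObject if already grabbed.
; Drop detaches it in place, with physics simulation kept off in both cases.
; setTextureKartu picks the material for mesh slot 1 from MerchantCardMaterials by index.
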(event `self.ReceiveBeginPlay`)

(event `/Game/Blueprint/PickupActorInterface.Pickup`
  (params (AttachTo :type "SceneComponent Object Reference"))
  (bind _returnvalue (select `bool` (`self.bSnapToSocket?`) :`false` "KeepWorld" :`true` "SnapToTarget" :!type "EAttachmentRule Enum"))
  (if (not (not (`self.bGrabbed?`)))
    (`/Game/Blueprint/BPC_PickupObject.Pickup` (`self.BPC_PickupObject`) AttachTo))
  (`PrimitiveComponent.SetSimulatePhysics` (`self.StaticMeshComponent`) false)
  (`SceneComponent.K2_AttachToComponent` (`self.RootComponent`) AttachTo (select `bool` (`self.bSnapToSocket?`) :`true` (`self.SnapSocket`)) _returnvalue _returnvalue "KeepWorld" false)
  (set `self.bGrabbed?` true))

(event `/Game/Blueprint/PickupActorInterface.Drop`
  (`PrimitiveComponent.SetSimulatePhysics` (`self.StaticMeshComponent`) false)
  (`self.K2_DetachFromActor` "KeepWorld" "KeepWorld" "KeepWorld")
  (set `self.bGrabbed?` false))

(event `setTextureKartu`
  (params (index :type Integer))
  (`PrimitiveComponent.SetMaterial` (`self.StaticMeshComponent`) 1 (`|GetArrayItem` (`self.MerchantCardMaterials`) index)))

(fn `GetAnimSequence`
  (params (Hand :type "EControllerHand Enum" :default "Left"))
  (returns (AnimSequence :type "AnimSequence Object Reference"))
  (return null))

(fn `GetPickupComponent`
  (returns (PickupComponent :type "/Game/Blueprint/BPC_PickupObject Object Reference"))
  (return (`self.Pickup Object`)))

(fn `UserConstructionScript`)