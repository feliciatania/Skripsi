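; Point-card exchange zone (Tukar Kartu Poin) that tallies and consumes gems (Permata) placed inside its Capsule.
; CheckPermata counts overlapping BP_Permata actors that have a valid OwnerPawn by sapphire, emerald or ruby tag and returns the totals as an SPermata struct.
; DestroyPermata destroys every overlapping gem regardless of owner, with debug prints.
; The event graph is empty, so both functions rely on external callers.
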(event `self.ReceiveBeginPlay`)

(fn `CheckPermata`
  (returns (Permatas :type "/Game/Blueprint/S_Permata Structure"))
  (bind _overlappingactors (`PrimitiveComponent.GetOverlappingActors` (`self.Capsule`) "/Game/Blueprint/BP_Permata.BP_Permata_C"))
  (set `self.count` (`KismetArrayLibrary.Array_Length` _overlappingactors))
  (set `self.Sapphire` 0)
  (set `self.Emerald` 0)
  (set `self.Ruby` 0)
  (for _array_element _overlappingactors
    (bind _asbp_permata (cast `/Game/Blueprint/BP_Permata` _array_element))
    (`/Game/Blueprint/BP_Permata.ownerPawn` _asbp_permata
      (:`then`
        (if (`self.ActorHasTag` _array_element "sapphire")
          (`/Engine/EditorBlueprintResources/StandardMacros.IncrementInt` (`self.Sapphire`))
          (elif (`self.ActorHasTag` _array_element "emerald")
            (`/Engine/EditorBlueprintResources/StandardMacros.IncrementInt` (`self.Emerald`))
            (elif (`self.ActorHasTag` _array_element "ruby")
              (`/Engine/EditorBlueprintResources/StandardMacros.IncrementInt` (`self.Ruby`))))))
      (:`else`)))
  (bind _output_get (set `self.SPermata` (make `/Game/Blueprint/S_Permata` (`self.Sapphire`) (`self.Emerald`) (`self.Ruby`))))
  (return _output_get))

(fn `DestroyPermata`
  (locals (Permatas :type "Array of Actor Object Reference"))
  (bind _overlappingactors (`PrimitiveComponent.GetOverlappingActors` (`self.Capsule`) "/Game/Blueprint/BP_Permata.BP_Permata_C"))
  (set `local.Permatas` _overlappingactors)
  (`KismetSystemLibrary.PrintString` (`KismetStringLibrary.Conv_IntToString` (`KismetArrayLibrary.Array_Length` _overlappingactors)))
  (for _array_element (`local.Permatas`)
    (`self.K2_DestroyActor` _array_element)
    (`KismetSystemLibrary.PrintString` "DESTROY"))
  (return))

(fn `UserConstructionScript`)