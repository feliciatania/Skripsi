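; BP_KartuPoin is a grabbable point card actor, identified by a card ID and showing a matching material.
; setKartu picks the material by index, and its RepNotify applies it to the mesh.
; Pickup attaches the card with optional socket snapping, routing through the pickup component if already held, while Drop detaches it with physics off.
; BeginPlay binds to a player state enable event, and SetCanGrab unlocks grabbing for a matching ID.
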(event `self.ReceiveBeginPlay`
  (bind _asbp_player_state (cast `/Game/Blueprint/BP_PlayerState` (`Controller.PlayerState` (`GameplayStatics.GetPlayerController` 0))))
  (add `/Game/Blueprint/BP_PlayerState.EnableKartuPoin` _asbp_player_state (`|CreateDelegate` :!event `SetCanGrab`)))

(event `/Game/Blueprint/PickupActorInterface.Pickup`
  (params (AttachTo :type "SceneComponent Object Reference"))
  (bind _returnvalue (select `bool` (`self.bSnapToSocket?`) :`false` "KeepWorld" :`true` "SnapToTarget" :!type "EAttachmentRule Enum"))
  (if (not (not (`self.bGrabbed?`)))
    (`/Game/Blueprint/BPC_PickupObject.Pickup` (`self.BPC_PickupObject`) AttachTo))
  (`PrimitiveComponent.SetSimulatePhysics` (`self.StaticMeshComponent`) false)
  (`SceneComponent.K2_AttachToComponent` (`self.RootComponent`) AttachTo (select `bool` (`self.bSnapToSocket?`) :`true` (`self.SnapSocket`)) _returnvalue _returnvalue "KeepWorld" false)
  (set `self.bGrabbed?` true))

(event `/Game/Blueprint/PickupActorInterface.Drop`
  (`PrimitiveComponent.SetSimulatePhysics` (`self.StaticMeshComponent`) false)
  (`self.K2_DetachFromActor` "KeepWorld" "KeepWorld" "KeepWorld")
  (set `self.bGrabbed?` false))

(event `setKartu`
  (params (index :type Integer))
  (set `self.TextureCard` (`|GetArrayItem` (`self.PoinCardMaterials`) index))
  (set `self.cardId` index))

(event `DisableCollision`
  (`PrimitiveComponent.SetCollisionEnabled` (`self.StaticMeshComponent`) "NoCollision"))

(event `EnableCollision`
  (`PrimitiveComponent.SetCollisionEnabled` (`self.StaticMeshComponent`) "QueryAndPhysics"))

(event `SetCanGrab`
  (params (enable :type Boolean) (id :type Integer))
  (if enable
    (if (== id (`self.cardId`))
      (set `self.CanGrab?` true))))

(fn `GetPickupComponent`
  (returns (PickupComponent :type "/Game/Blueprint/BPC_PickupObject Object Reference"))
  (return (`self.Pickup Object`)))

(fn `OnRep_cardId`)

(fn `OnRep_Index`)

(fn `OnRep_TextureCard`
  (`PrimitiveComponent.SetMaterial` (`self.StaticMeshComponent`) 2 (`self.TextureCard`)))

(fn `UserConstructionScript`)