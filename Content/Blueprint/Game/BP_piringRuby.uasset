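; BP_piringRuby is a plate actor that catches and tallies ruby gems (BP_PermataRuby).
; Its Box overlap calls EnablePhysic(false) on any arriving BP_Permata tagged "permata".
; Helper functions count rubies in the Box, count those overlapping Piring with a valid OwnerPawn, and clear OwnerPawn on the Box's rubies.
; The clearing loop returns after the first successful cast, so it releases only one gem per call.
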(event `self.ReceiveBeginPlay`)

(event `self.Box.OnComponentBeginOverlap`
  (params (OverlappedComponent :type "PrimitiveComponent Object Reference") (OtherActor :type "Actor Object Reference") (OtherComp :type "PrimitiveComponent Object Reference") (OtherBodyIndex :type Integer) (bFromSweep :type Boolean) (SweepResult :type "HitResult Structure (by ref)"))
  (if (`self.ActorHasTag` OtherActor "permata")
    (bind _asbp_permata (cast `/Game/Blueprint/BP_Permata` OtherActor))
    (`/Game/Blueprint/BP_Permata.EnablePhysic` _asbp_permata false)))

(fn `GetCountPermata`
  (returns (count :type Integer))
  (return (`KismetArrayLibrary.Array_Length` (`PrimitiveComponent.GetOverlappingActors` (`self.Box`) "/Game/Blueprint/Game/BP_PermataRuby.BP_PermataRuby_C"))))

(fn `GetCountPermataPlayer`
  (returns (count :type Integer))
  (locals (counter :type Integer) (permatas :type "Array of Actor Object Reference"))
  (bind _output_get (set `local.permatas` (`PrimitiveComponent.GetOverlappingActors` (`self.piring`) "/Game/Blueprint/Game/BP_PermataRuby.BP_PermataRuby_C")))
  (for _array_element _output_get
    (bind _asbp_permata (cast `/Game/Blueprint/BP_Permata` _array_element))
    (`/Game/Blueprint/BP_Permata.ownerPawn` _asbp_permata
      (:`then`
        (`/Engine/EditorBlueprintResources/StandardMacros.IncrementInt` (`local.counter`)))
      (:`else`)))
  (return (`local.counter`)))

(fn `SetOwnerPawnToNone`
  (for _array_element (`PrimitiveComponent.GetOverlappingActors` (`self.Box`) "/Game/Blueprint/Game/BP_PermataRuby.BP_PermataRuby_C")
    (bind _asbp_permata (cast `/Game/Blueprint/BP_Permata` _array_element))
    (set `/Game/Blueprint/BP_Permata.ownerPawn` null _asbp_permata)
    (return)))

(fn `UserConstructionScript`)