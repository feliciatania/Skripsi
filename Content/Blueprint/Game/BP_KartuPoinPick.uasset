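; BP_KartuPoinPick is an actor that, judging by its name, represents a point card that can be picked up and dropped.
; On BeginPlay it calls the parent logic and turns physics simulation off on its static mesh.
; Its Drop event disables physics again and detaches the actor while keeping its world transform, with no pickup or scoring logic in this graph.
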(event `self.ReceiveBeginPlay`
  (`parent.ReceiveBeginPlay`)
  (`PrimitiveComponent.SetSimulatePhysics` (`self.StaticMeshComponent`) false))

(event `/Game/Blueprint/PickupActorInterface.Drop`
  (`PrimitiveComponent.SetSimulatePhysics` (`self.StaticMeshComponent`) false)
  (`self.K2_DetachFromActor` "KeepWorld" "KeepWorld" "KeepWorld"))

(fn `UserConstructionScript`
  (`parent.UserConstructionScript`))