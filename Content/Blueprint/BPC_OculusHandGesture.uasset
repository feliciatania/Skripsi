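; Oculus hand component that records, saves and recognises named hand gestures as component-space bone-location snapshots.
; Recording and deletion update a GestureSaveGame slot, and BeginPlay loads the saved list.
; A looping timer selects the first gesture whose bones all lie within a distance threshold, firing OnGestureRecognised when it differs from the current one.
; Losing a match leaves the current gesture set, so repeating it does not refire the event.
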(event `self.ReceiveBeginPlay`
  (set `self.Gestures` (`/Game/Blueprint/GestureSaveGame.Gestures` (`self.LoadGestures`)))
  (`KismetSystemLibrary.K2_SetTimerDelegate` (delegate `DetectGesture`) (`self.RefreshRate`) true))

(event `DetectGesture`
  (bind (_gesturefound _gesture) (`self.GetCurrentGesture`))
  (if _gesturefound
    (if (not (`self.GestureEqual` _gesture (`self.CurrentGesture`)))
      (bind _output_get (set `self.CurrentGesture` _gesture))
      (`self.OnGestureRecognised` (`.GestureName_3_469017594D6BABBA6AB4B1B53C406914` (break `/Game/Blueprint/S_Gesture` _output_get))))))

(fn `DeleteGesture`
  (params (GestureName :type String))
  (locals (GestureSaveGame :type "/Game/Blueprint/GestureSaveGame Object Reference") (Index :type Integer))
  (bind _output_get (set `local.GestureSaveGame` (`self.LoadGestures`)))
  (bind _gestures (`/Game/Blueprint/GestureSaveGame.Gestures` _output_get))
  (for (_array_element _array_index) _gestures
    (if (`KismetStringLibrary.EqualEqual_StrStr` (`.GestureName_3_469017594D6BABBA6AB4B1B53C406914` (break `/Game/Blueprint/S_Gesture` _array_element)) GestureName)
      (set `local.Index` _array_index)))
  (`KismetArrayLibrary.Array_Remove` _gestures (`local.Index`))
  (`GameplayStatics.SaveGameToSlot` (`local.GestureSaveGame`) (`self.GestureGameSlot`)))

(fn `DoesGestureAlreadyExist?`
  (params (SaveGame :type "/Game/Blueprint/GestureSaveGame Object Reference") (GestureName :type String))
  (returns (ResultValue :type Boolean))
  (for _array_element (`/Game/Blueprint/GestureSaveGame.Gestures` SaveGame)
    (if (`KismetStringLibrary.EqualEqual_StrStr` (`.GestureName_3_469017594D6BABBA6AB4B1B53C406914` (break `/Game/Blueprint/S_Gesture` _array_element)) GestureName)
      (return true)))
  (return false))

(fn `GestureEqual`
  (params (A :type "/Game/Blueprint/S_Gesture Structure") (B :type "/Game/Blueprint/S_Gesture Structure"))
  (returns (ReturnValue :type Boolean))
  (bind (_gesturename _bonelocations) (break `/Game/Blueprint/S_Gesture` A))
  (bind (_gesturename_2 _bonelocations_2) (break `/Game/Blueprint/S_Gesture` B))
  (return (and (`KismetStringLibrary.EqualEqual_StrStr` _gesturename _gesturename_2) (`KismetArrayLibrary.Array_Identical` _bonelocations _bonelocations_2))))

(fn `GetCurrentGesture`
  (returns (GestureFound :type Boolean) (Gesture :type "/Game/Blueprint/S_Gesture Structure"))
  (locals (bValidGesture :type Boolean :default true))
  (for _array_element (`self.Gestures`)
    (for (_array_element_2 _array_index) (`.BoneLocations_9_0D6F4B154407E2C1275443AB1E961E47` (break `/Game/Blueprint/S_Gesture` _array_element))
      (bind _returnvalue (`self.GetBoneLocationByName` (`self.GetBoneName` _array_index) "ComponentSpace"))
      (if (`self.bDebug`)
        (bind _returnvalue_2 (`KismetMathLibrary.Abs` (`KismetMathLibrary.VSize` (- _returnvalue _array_element_2))))
        (`KismetSystemLibrary.PrintString` (`KismetStringLibrary.Conv_DoubleToString` _returnvalue_2)))
      (if (> _returnvalue_2 (`self.Threshold`))
        (set `local.bValidGesture` false)))
    (if (`local.bValidGesture`)
      (return (`local.bValidGesture`) _array_element)
      (else
        (set `local.bValidGesture` true))))
  (return false))

(fn `LoadGestures`
  (returns (Output_Get :type "/Game/Blueprint/GestureSaveGame Object Reference"))
  (locals (GestureSaveGame :type "/Game/Blueprint/GestureSaveGame Object Reference"))
  (bind _returnvalue (`GameplayStatics.DoesSaveGameExist` (`self.GestureGameSlot`)))
  (`KismetSystemLibrary.PrintString` (`KismetStringLibrary.Conv_BoolToString` _returnvalue))
  (if _returnvalue
    (bind _returnvalue_2 (`GameplayStatics.LoadGameFromSlot` (`self.GestureGameSlot`)))
    (bind _asgesture_save_game (cast `/Game/Blueprint/GestureSaveGame` _returnvalue_2))
    (set `local.GestureSaveGame` _asgesture_save_game)
    (else
      (bind _returnvalue_3 (`GameplayStatics.CreateSaveGameObject` "/Game/Blueprint/GestureSaveGame.GestureSaveGame_C"))
      (set `local.GestureSaveGame` _returnvalue_3)))
  (return (`local.GestureSaveGame`)))

(fn `RecordGesture`
  (params (GestureName :type String))
  (locals (GestureSaveGame :type "/Game/Blueprint/GestureSaveGame Object Reference") (BoneLocations :type "Array of Vector Structure"))
  (bind _output_get (set `local.GestureSaveGame` (`self.LoadGestures`)))
  (if (not (`self.DoesGestureAlreadyExist?` _output_get GestureName))
    (for _index (range (`self.GetNumBones`))
      (bind _returnvalue (`self.GetBoneLocationByName` (`self.GetBoneName` _index) "ComponentSpace"))
      (`KismetArrayLibrary.Array_Add` (`local.BoneLocations`) _returnvalue))
    (`KismetArrayLibrary.Array_Add` (`/Game/Blueprint/GestureSaveGame.Gestures` (`local.GestureSaveGame`)) (make `/Game/Blueprint/S_Gesture` (`local.GestureName`) (`local.BoneLocations`)))
    (`GameplayStatics.SaveGameToSlot` (`local.GestureSaveGame`) (`self.GestureGameSlot`))))